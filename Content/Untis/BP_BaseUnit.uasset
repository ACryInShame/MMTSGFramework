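; Base unit Blueprint that fits its selection capsule to its skeletal mesh and takes damage when clicked.
; On BeginPlay it scales the mesh bounds by a selection factor, using the larger horizontal extent as capsule radius and the vertical as half-height.
; Invalid capsule or mesh references print an error instead.
; Clicking applies fixed damage and prints current health, apparently as a debug test.
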(event `self.ReceiveBeginPlay`
  (`self.ResizeCapsuleToSkeleton`))

(event `self.ReceiveActorOnClicked`
  (params (ButtonPressed :type "Key Structure"))
  (`self.TakeDamage` 10)
  (`KismetSystemLibrary.PrintString` (`KismetStringLibrary.Conv_IntToString` (`self.CurrentHealth`)) true true (struct :`G` 0.66 :`B` 1.0 :`A` 1.0) 5.0))

(fn `ResizeCapsuleToSkeleton`
  (bind _capsule (`self.Capsule`))
  (bind _selection_compnent_scale (`self.Selection Compnent Scale`))
  (bind (_returnvalue_x _returnvalue_y _returnvalue_z) (`KismetMathLibrary.BreakVector` (* (`.BoxExtent` (`KismetSystemLibrary.GetComponentBounds` (`self.Skeletal Mesh`))) (`KismetMathLibrary.MakeVector` _selection_compnent_scale _selection_compnent_scale _selection_compnent_scale))))
  (`/Engine/EditorBlueprintResources/StandardMacros.IsValid` (`self.Capsule`)
    (:`Is Valid`
      (`/Engine/EditorBlueprintResources/StandardMacros.IsValid` (`self.Skeletal Mesh`)
        (:`Is Valid`
          (`CapsuleComponent.SetCapsuleSize` _capsule (`KismetMathLibrary.FMax` _returnvalue_x _returnvalue_y) _returnvalue_z true)
          (`SceneComponent.K2_AddLocalOffset` _capsule (0.0 0.0 0.0) false false))
        (:`Is Not Valid`
          (`KismetSystemLibrary.PrintString` "Unit Skeltal Mesh Invalud")
          (return))))
    (:`Is Not Valid`
      (`KismetSystemLibrary.PrintString` "Unit SelectionColider not valid")
      (return))))

(fn `UserConstructionScript`)