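; Player controller for battle play that sets up Enhanced Input controls, the game HUD and a toggleable player menu.
; On BeginPlay it adds the battle mapping context, creates both widgets, caches the camera pawn and HUD selection panels, and enables mouse cursor clicks.
; Input actions forward move, rotate and zoom to P_PlayerCamera, and left click to HandleMouseClick.
; Toggling the menu switches input mode, forcing garbage collection on close.
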(event `self.ReceiveBeginPlay`
  (bind _returnvalue (subsystem `EnhancedInputLocalPlayerSubsystem`))
  (bind _playerhud (`self.PlayerHUD`))
  ; Set Default Controls for player
  (`/Engine/EditorBlueprintResources/StandardMacros.IsValid` _returnvalue
    (:`Is Valid`
      (`EnhancedInputSubsystemInterface.AddMappingContext` _returnvalue "/Game/Player/Controls/ActionMaps/IM_PlayerBattleControls.IM_PlayerBattleControls" 0 (struct))
      (`EnhancedInputSubsystemInterface.AddMappingContext` _returnvalue "/Game/Player/Controls/ActionMaps/IM_PlayerBattleControls.IM_PlayerBattleControls" 0 (struct))
      (`self.CreatePlayerWidgets`)
      (`UserWidget.AddToViewport` (`self.PlayerHUD`) 0)
      (set `self.Player Camera` (cast `/Game/Player/P_PlayerCamera` (`GameplayStatics.GetPlayerPawn` 0) :!pure true))
      (set `self.MovingCamera` true)
      (`WidgetBlueprintLibrary.SetInputMode_GameAndUIEx` self (`self.PlayerHUD`) "DoNotLock" false)
      (set `self.bShowMouseCursor` true)
      (set `self.bEnableClickEvents` true)
      (set `self.UnitSelectionWidget` (`/Game/UI/UI_Huds/W_GameHUD.W_UnitSelectionInfo` _playerhud))
      (set `self.TileSelectionWidget` (`/Game/UI/UI_Huds/W_GameHUD.W_TileSelectionInfo` _playerhud)))))

(event `EnhancedInput|/Game/Player/Controls/Actions/IA_MenuOpen`
  (params (ActionValue :type Boolean) (ElapsedSeconds :type "Float (double-precision)") (TriggeredSeconds :type "Float (double-precision)") (InputAction :type "InputAction Object Reference" :default "/Game/Player/Controls/Actions/IA_MenuOpen.IA_MenuOpen"))
  (:`Started`
    (`self.ToggleMenu`)))

(event `EnhancedInput|/Game/Player/Controls/Actions/IA_CameraMove`
  (params (ActionValue :type "Vector2D Structure") (ElapsedSeconds :type "Float (double-precision)") (TriggeredSeconds :type "Float (double-precision)") (InputAction :type "InputAction Object Reference" :default "/Game/Player/Controls/Actions/IA_CameraMove.IA_CameraMove"))
  (:`Triggered`
    (if (`self.MovingCamera`)
      (`PlayerCamera.MoveCamera` (`self.Player Camera`) ActionValue))))

(event `EnhancedInput|/Game/Player/Controls/Actions/IA_CameraRotate`
  (params (ActionValue :type "Float (double-precision)") (ElapsedSeconds :type "Float (double-precision)") (TriggeredSeconds :type "Float (double-precision)") (InputAction :type "InputAction Object Reference" :default "/Game/Player/Controls/Actions/IA_CameraRotate.IA_CameraRotate"))
  (:`Triggered`
    (`PlayerCamera.RotateCamera` (`self.Player Camera`) ActionValue)))

(event `EnhancedInput|/Game/Player/Controls/Actions/IA_CameraZoom`
  (params (ActionValue :type "Float (double-precision)") (ElapsedSeconds :type "Float (double-precision)") (TriggeredSeconds :type "Float (double-precision)") (InputAction :type "InputAction Object Reference" :default "/Game/Player/Controls/Actions/IA_CameraZoom.IA_CameraZoom"))
  (:`Triggered`
    (`PlayerCamera.ZoomCamera` (`self.Player Camera`) ActionValue)))

(event `EnhancedInput|/Game/Player/Controls/Actions/IA_LeftMouseClick`
  (params (ActionValue :type Boolean) (ElapsedSeconds :type "Float (double-precision)") (TriggeredSeconds :type "Float (double-precision)") (InputAction :type "InputAction Object Reference" :default "/Game/Player/Controls/Actions/IA_LeftMouseClick.IA_LeftMouseClick"))
  (:`Triggered`
    (`self.HandleMouseClick`)))

(fn `CreatePlayerWidgets`
  (bind _returnvalue (`|CreateWidget` "/Game/UI/UI_Menus/W_PlayerMenu.W_PlayerMenu_C"))
  (set `self.PlayerMenu` _returnvalue)
  (bind _returnvalue_2 (`|CreateWidget` "/Game/UI/UI_Huds/W_GameHUD.W_GameHUD_C"))
  (set `self.PlayerHUD` _returnvalue_2))

(fn `ToggleMenu`
  (bind _playermenu (`self.PlayerMenu`))
  ;[1 1 1] Toggles show/hide of supplied Menu Widget
  (if (`GameViewportSubsystem.IsWidgetAdded` (subsystem `GameViewportSubsystem`) (`self.PlayerMenu`))
    (`GameViewportSubsystem.RemoveWidget` (subsystem `GameViewportSubsystem`) _playermenu)
    (`KismetSystemLibrary.CollectGarbage`)
    (`WidgetBlueprintLibrary.SetInputMode_GameOnly` self true)
    (else
      (`UserWidget.AddToViewport` _playermenu 0)
      (`WidgetBlueprintLibrary.SetInputMode_GameAndUIEx` self null))))

(fn `UserConstructionScript`)