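; Player controller that sets up Enhanced Input and owns the player's HUD and toggleable menu widgets.
; BeginPlay adds the IM_PlayerMenu mapping context (twice), creates both widgets and shows the HUD.
; IA_OpenMenu calls ToggleMenu, which adds or removes the menu, switching input mode and cursor visibility, with garbage collection on close.
; An unconnected owner-check setup chain remains in the graph and never runs.
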(event `self.ReceiveBeginPlay`
  (bind _returnvalue (subsystem `EnhancedInputLocalPlayerSubsystem`))
  ; Set Default Controls for player
  (`/Engine/EditorBlueprintResources/StandardMacros.IsValid` _returnvalue
    (:`Is Valid`
      (`EnhancedInputSubsystemInterface.AddMappingContext` _returnvalue "/Game/Controls/ActionMaps/IM_PlayerMenu.IM_PlayerMenu" 0 (struct))
      (`EnhancedInputSubsystemInterface.AddMappingContext` _returnvalue "/Game/Controls/ActionMaps/IM_PlayerMenu.IM_PlayerMenu" 0 (struct))
      (`self.CreatePlayerWidgets`)
      (`UserWidget.AddToViewport` (`self.PlayerHUD`) 0))))

(event `EnhancedInput|/Game/Controls/Actions/IA_OpenMenu`
  (params (ActionValue :type Boolean) (ElapsedSeconds :type "Float (double-precision)") (TriggeredSeconds :type "Float (double-precision)") (InputAction :type "InputAction Object Reference" :default "/Game/Controls/Actions/IA_OpenMenu.IA_OpenMenu"))
  (:`Started`
    (`self.ToggleMenu`)))

(fn `CreatePlayerWidgets`
  (bind _returnvalue (`|CreateWidget` "/Game/UI/UI_Menus/W_PlayerMenu.W_PlayerMenu_C"))
  (set `self.PlayerMenu` _returnvalue)
  (bind _returnvalue_2 (`|CreateWidget` "/Game/UI/UI_Huds/W_GameHUD.W_GameHUD_C"))
  (set `self.PlayerHUD` _returnvalue_2))

(fn `ToggleMenu`
  (bind _playermenu (`self.PlayerMenu`))
  ;[1 1 1] Toggles show/hide of supplied Menu Widget
  (if (`GameViewportSubsystem.IsWidgetAdded` (subsystem `GameViewportSubsystem`) (`self.PlayerMenu`))
    (`GameViewportSubsystem.RemoveWidget` (subsystem `GameViewportSubsystem`) _playermenu)
    (`KismetSystemLibrary.CollectGarbage`)
    (`WidgetBlueprintLibrary.SetInputMode_GameOnly` self true)
    (set `self.bShowMouseCursor` false)
    (else
      (`UserWidget.AddToViewport` _playermenu 0)
      (`WidgetBlueprintLibrary.SetInputMode_GameAndUIEx` self null)
      (set `self.bShowMouseCursor` true))))

(fn `UserConstructionScript`)