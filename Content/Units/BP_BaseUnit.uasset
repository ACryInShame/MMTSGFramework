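; BP_BaseUnit is a base unit Blueprint with logic meant to fit a selection capsule to its skeletal mesh.
; BeginPlay calls ResizeCapsuleToSkeleton, but that function's body is disconnected from its entry, so nothing is resized.
; The unused nodes validate components, derive capsule radius and half-height from scaled mesh bounds, then apply a local offset.
; The click event is empty.
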(event `self.ReceiveBeginPlay`
  (`self.ResizeCapsuleToSkeleton`))

(event `self.ReceiveActorOnClicked`
  (params (ButtonPressed :type "Key Structure")))

(fn `ResizeCapsuleToSkeleton`)

(fn `UserConstructionScript`)